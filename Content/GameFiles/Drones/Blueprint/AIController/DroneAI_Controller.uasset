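; AI controller for enemy drones that runs their behavior tree and drives Patrol, Investigate and Chase states from perception.
; Stimuli from Player and Distract actors dispatch by array index to sight, hearing and damage handlers; Distract skips sight.
; Sight starts a faster chase; losing it saves the player's location and investigates, returning to patrol after a delay.
; Fire or distraction noises, and damage while patrolling, trigger investigation focused on the stimulus.
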(event OnPerceptionUpdated(AIPerception)
  (params (UpdatedActors :type Array%20of%20Actor%20Object%20References))
  (for _array_element UpdatedActors
    (if (Actor|ActorHasTag _array_element "Player")
      (bind _info (Class|AIPerceptionComponent|GetActorsPerception (Variables|Default|GetAIPerception) _array_element))
      (for (_array_element_2 _array_index) (.lastsensedstimuli _info)
        (bind _output_get (Variables|Default|SetActiveSense _array_element_2))
        (Variables|Default|SetStimulus%20Location (.StimulusLocation (Utilities|Struct|BreakAIStimulus _output_get)))
        (Variables|Default|SetReceiver%20Location (.ReceiverLocation (Utilities|Struct|BreakAIStimulus _output_get)))
        (switch int _array_index
          (:0
            (CallFunction|SightSense))
          (:1
            (CallFunction|HearingSense))
          (:2
            (CallFunction|DamageSense))))
      (elif (Actor|ActorHasTag _array_element "Distract")
        (bind _info_2 (Class|AIPerceptionComponent|GetActorsPerception (Variables|Default|GetAIPerception)))
        (for (_array_element_3 _array_index_2) (.lastsensedstimuli _info_2)
          (bind _output_get_2 (Variables|Default|SetActiveSense _array_element_3))
          (Variables|Default|SetStimulus%20Location (.StimulusLocation (Utilities|Struct|BreakAIStimulus _output_get_2)))
          (Variables|Default|SetReceiver%20Location (.ReceiverLocation (Utilities|Struct|BreakAIStimulus _output_get_2)))
          (switch int _array_index_2
            (:1
              (CallFunction|HearingSense))
            (:2
              (CallFunction|DamageSense))))))))

(event Custom|SightSense
  (if (.bSuccessfullySensed (Utilities|Struct|BreakAIStimulus (Variables|Default|GetActiveSense)))
    (switch Utilities|FlowControl|Switch|SwitchonDroneAI_States (Variables|/Game/GameFiles/Drones/Blueprint/BP_Drone_Base.BP_Drone_Base_C|GetAIState (Variables|Default|GetDroneAIRef))
      (:NewEnumerator0
        _)
      (:NewEnumerator5
        _))
    (Variables|/Game/GameFiles/Drones/Blueprint/BP_Drone_Base.BP_Drone_Base_C|SetAIState (Variables|Default|GetDroneAIRef) "NewEnumerator1")
    (Variables|/Script/Engine.CharacterMovementComponent|SetMaxFlySpeed (Variables|/Script/Engine.Character|GetCharacterMovement (Variables|Default|GetDroneAIRef)) 6e+02)
    (else
      (switch Utilities|FlowControl|Switch|SwitchonDroneAI_States (Variables|/Game/GameFiles/Drones/Blueprint/BP_Drone_Base.BP_Drone_Base_C|GetAIState (Variables|Default|GetDroneAIRef))
        (:NewEnumerator1
          (Variables|/Game/GameFiles/Drones/Blueprint/BP_Drone_Base.BP_Drone_Base_C|SetAIState (Variables|Default|GetDroneAIRef) "NewEnumerator5")
          (Variables|/Game/GameFiles/Drones/Blueprint/BP_Drone_Base.BP_Drone_Base_C|SetPlayerLastSeenLocation (Variables|Default|GetDroneAIRef) (Transformation|GetActorLocation (Variables|/Game/GameFiles/Drones/Blueprint/BP_Drone_Base.BP_Drone_Base_C|GetPlayerRef (Variables|Default|GetDroneAIRef))))
          (Variables|/Script/Engine.CharacterMovementComponent|SetMaxFlySpeed (Variables|/Script/Engine.Character|GetCharacterMovement (Variables|Default|GetDroneAIRef)) 4e+02)
          (Utilities|FlowControl|Delay 2e+01)
          (if (Utilities|Enum|Equal(Enum) (Variables|/Game/GameFiles/Drones/Blueprint/BP_Drone_Base.BP_Drone_Base_C|GetAIState (Variables|Default|GetDroneAIRef)) "NewEnumerator5")
            (Variables|/Game/GameFiles/Drones/Blueprint/BP_Drone_Base.BP_Drone_Base_C|SetAIState (Variables|Default|GetDroneAIRef) "NewEnumerator0")
            (Variables|/Script/Engine.CharacterMovementComponent|SetMaxFlySpeed (Variables|/Script/Engine.Character|GetCharacterMovement (Variables|Default|GetDroneAIRef)) 2e+02)))))))

(event Custom|HearingSense
  (bind _activesense (Variables|Default|GetActiveSense))
  (bind (_age _expirationage _strength _stimuluslocation _receiverlocation _tag _bsuccessfullysensed) (Utilities|Struct|BreakAIStimulus _activesense))
  (if _bsuccessfullysensed
    (bind _output_get (Variables|Default|SetNoiseTag _tag))
    (if (Utilities|Name|Equal(Name) _output_get "FireNoise")
      (switch Utilities|FlowControl|Switch|SwitchonDroneAI_States (Variables|/Game/GameFiles/Drones/Blueprint/BP_Drone_Base.BP_Drone_Base_C|GetAIState (Variables|Default|GetDroneAIRef)) :!label _label
        (:NewEnumerator0
          _)
        (:NewEnumerator5
          _))
      (Variables|/Game/GameFiles/Drones/Blueprint/BP_Drone_Base.BP_Drone_Base_C|SetAIState (Variables|Default|GetDroneAIRef) "NewEnumerator5")
      (AI|SetFocalPoint (Variables|Default|GetStimulus%20Location))
      (elif (Utilities|Name|Equal(Name) _output_get "Distract")
        (goto _label)))))

(event Custom|DamageSense
  (if (.bSuccessfullySensed (Utilities|Struct|BreakAIStimulus (Variables|Default|GetActiveSense)))
    (switch Utilities|FlowControl|Switch|SwitchonDroneAI_States (Variables|/Game/GameFiles/Drones/Blueprint/BP_Drone_Base.BP_Drone_Base_C|GetAIState (Variables|Default|GetDroneAIRef))
      (:NewEnumerator0
        (Variables|/Game/GameFiles/Drones/Blueprint/BP_Drone_Base.BP_Drone_Base_C|SetAIState (Variables|Default|GetDroneAIRef) "NewEnumerator5")
        (AI|SetFocalPoint (Variables|Default|GetStimulus%20Location))))))

(event EventBeginPlay
  (AI|RunBehaviorTree "/Game/GameFiles/Drones/Blueprint/AIController/BT_DroneAI.BT_DroneAI")
  (bind _asbp_drone_base (Utilities|Casting|CastToBP_Drone_Base (Pawn|GetControlledPawn)))
  (Variables|Default|SetDroneAIRef _asbp_drone_base))

(fn ConstructionScript)