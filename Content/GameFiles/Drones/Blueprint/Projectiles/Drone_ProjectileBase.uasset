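; Base Blueprint for drone projectiles, handling impact effects and damage to the player.
; Its Hit event stores the hit data, disables and hides the collision sphere, then spawns an impact particle chosen by physical surface type.
; The projectile destroys itself after a short delay, while a parallel sequence branch sends a damage message with bone and location to actors tagged Player.
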(event EventBeginPlay)

(event Collision|EventActorBeginOverlap
  (params (OtherActor :type Actor%20Object%20Reference)))

(event EventTick
  (params (DeltaSeconds :type Float%20%28single-precision%29)))

(event Collision|EventHit
  (params (MyComp :type Primitive%20Component%20Object%20Reference) (Other :type Actor%20Object%20Reference) (OtherComp :type Primitive%20Component%20Object%20Reference) (bSelfMoved :type Boolean) (HitLocation :type Vector :default "0, 0, 0") (HitNormal :type Vector :default "0, 0, 0") (NormalImpulse :type Vector :default "0, 0, 0") (Hit :type Hit%20Result%20Structure%20%28by%20ref%29))
  (Variables|Default|SetHit%20Location HitLocation)
  (Variables|Default|SetHit Hit)
  (Collision|SetCollisionEnabled (Variables|Default|GetSphere) "NoCollision")
  (Rendering|SetVisibility (Variables|Default|GetSphere) false true)
  (Utilities|FlowControl|Sequence
    (:then_0
      (Effects|SpawnEmitteratLocation (Utilities|Select :Index (Variables|/Script/PhysicsCore.PhysicalMaterial|GetSurfaceType (.PhysMat (Collision|BreakHitResult (Variables|Default|GetHit)))) :SurfaceType_Default "/Game/Assets/MilitaryWeapDark/FX/P_Impact_Metal_Medium_01.P_Impact_Metal_Medium_01" :SurfaceType1 "/Game/Assets/MilitaryWeapDark/FX/P_Impact_Stone_Medium_01.P_Impact_Stone_Medium_01" :SurfaceType2 "/Game/Assets/MilitaryWeapDark/FX/P_Impact_Wood_Medium_01.P_Impact_Wood_Medium_01" :SurfaceType3 "/Game/GameFiles/Blueprint/Weapons/ImpactEffects/Effects/Sparks/P_body_bullet_impact.P_body_bullet_impact" :SurfaceType4 "/Game/GameFiles/Blueprint/Weapons/ImpactEffects/Effects/Sparks/P_body_bullet_impact.P_body_bullet_impact" :SurfaceType5 "/Game/GameFiles/Blueprint/Weapons/ImpactEffects/Effects/Sparks/P_body_bullet_impact.P_body_bullet_impact" :SurfaceType6 0 :SurfaceType7 "/Game/Assets/MilitaryWeapDark/FX/P_Impact_Wood_Medium_01.P_Impact_Wood_Medium_01" :SurfaceType8 0 :SurfaceType9 0 :SurfaceType10 0 :SurfaceType11 0) (Variables|Default|GetHit%20Location))
      (Utilities|FlowControl|Delay 0.1)
      (Actor|DestroyActor))
    (:then_1
      (if (Actor|ActorHasTag (.HitActor (Collision|BreakHitResult (Variables|Default|GetHit))) "Player")
        (Class|DamageInterface|Damage(Message) (.HitActor (Collision|BreakHitResult (Variables|Default|GetHit))) 1.0 "NewEnumerator0" (.HitBoneName (Collision|BreakHitResult (Variables|Default|GetHit))) "0, 0, 0" (Variables|Default|GetHit%20Location))))))

(fn ConstructionScript)