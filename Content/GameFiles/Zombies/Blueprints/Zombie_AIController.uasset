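; AI controller for zombies that uses sight perception of Player-tagged actors to set the controlled zombie's state.
; Sighting switches it to chase after a short random delay, losing sight returns it to idle, and dead zombies stay dead.
; An idle roam routine nudges the zombie toward random nearby points, but its CustomTick timer is unwired, as is the behavior tree launch.
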(event OnPerceptionUpdated(AIPerception)
  (params (UpdatedActors :type Array%20of%20Actor%20Object%20References))
  (if (Utilities|Enum|NotEqual(Enum) (Variables|/Game/GameFiles/Zombies/Blueprints/ZombieCharacter_Base.ZombieCharacter_Base_C|GetZombieState (Variables|Default|GetZombieRef)) "NewEnumerator3")
    (for _array_element UpdatedActors
      (if (Actor|ActorHasTag _array_element "Player")
        (bind _info (Class|AIPerceptionComponent|GetActorsPerception (Variables|Default|GetAIPerception) _array_element))
        (for (_array_element_2 _array_index) (.lastsensedstimuli _info)
          (bind _output_get (Variables|Default|SetActiveSense _array_element_2))
          (Variables|Default|SetStimulus%20Location (.StimulusLocation (Utilities|Struct|BreakAIStimulus _output_get)))
          (Variables|Default|SetReceiver%20Location (.ReceiverLocation (Utilities|Struct|BreakAIStimulus _output_get)))
          (if (Variables|/Game/GameFiles/Zombies/Blueprints/ZombieCharacter_Base.ZombieCharacter_Base_C|GetIsDead (Variables|Default|GetZombieRef))
            (Variables|/Game/GameFiles/Zombies/Blueprints/ZombieCharacter_Base.ZombieCharacter_Base_C|SetZombieState (Variables|Default|GetZombieRef) "NewEnumerator3")
            (else
              (switch int _array_index
                (:0
                  (CallFunction|SightSense))))))))))

(event Custom|SightSense
  (if (.bSuccessfullySensed (Utilities|Struct|BreakAIStimulus (Variables|Default|GetActiveSense)))
    (Utilities|FlowControl|Delay (Math|Random|RandomFloatinRange 0.2 1.2))
    (Variables|/Game/GameFiles/Zombies/Blueprints/ZombieCharacter_Base.ZombieCharacter_Base_C|SetZombieState (Variables|Default|GetZombieRef) "NewEnumerator1")
    (else
      (switch Utilities|FlowControl|Switch|SwitchonZombieState (Variables|/Game/GameFiles/Zombies/Blueprints/ZombieCharacter_Base.ZombieCharacter_Base_C|GetZombieState (Variables|Default|GetZombieRef))
        (:NewEnumerator1
          (Utilities|FlowControl|Delay 1.0)
          (Variables|/Game/GameFiles/Zombies/Blueprints/ZombieCharacter_Base.ZombieCharacter_Base_C|SetZombieState (Variables|Default|GetZombieRef) "NewEnumerator0"))))))

(event Custom|CustomTick
  (switch Utilities|FlowControl|Switch|SwitchonZombieState (Variables|/Game/GameFiles/Zombies/Blueprints/ZombieCharacter_Base.ZombieCharacter_Base_C|GetZombieState (Variables|Default|GetZombieRef))
    (:NewEnumerator0
      (CallFunction|ZombieIdle))))

(event EventBeginPlay
  (bind _aszombie_character_base (Utilities|Casting|CastToZombieCharacter_Base (Pawn|GetControlledPawn)))
  (Variables|Default|SetZombieRef _aszombie_character_base))

(event EventTick
  (params (DeltaSeconds :type Float%20%28single-precision%29)))

(event Custom|ZombieIdle
  (bind _zombieref (Variables|Default|GetZombieRef))
  (bind _zombieref_2 (Variables|Default|GetZombieRef))
  (bind _returnvalue (Transformation|GetActorLocation _zombieref_2))
  (bind _returnvalue_2 (Transformation|GetActorLocation _zombieref))
  (if (not (Variables|Default|GetIsRoaming))
    (bind _output_get (Variables|Default|SetRoamLocation (Math|Vector|MakeVector (+ (.x _returnvalue) (Math|Random|RandomFloatinRange -1e+02 1e+02)) (+ (.y _returnvalue) (Math|Random|RandomFloatinRange -1e+02 1e+02)) (.z _returnvalue))))
    (Variables|Default|SetIsRoaming true)
    (Pawn|Input|AddMovementInput _zombieref (Math|Vector|GetUnitDirection(Vector) _returnvalue_2 _output_get) 1.0 false)
    (Transformation|SetActorRotation (Variables|Default|GetZombieRef) (Math|Rotator|FindLookatRotation _returnvalue_2 _output_get))
    (Utilities|FlowControl|Delay (Math|Random|RandomFloatinRange 1.0 5.0))
    (Variables|Default|SetIsRoaming false)))

(fn ConstructionScript)