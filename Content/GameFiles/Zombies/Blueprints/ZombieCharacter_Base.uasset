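; Base zombie character with a random mesh that roams when idle, chases and attacks the player, and ragdolls on death.
; Tick switches on ZombieState to set speed and steer by direct movement input, destroying corpses not recently rendered.
; Forward sphere traces flag the player in melee range and detect ledges, choosing between two mantle montages played in flying mode without capsule collision.
; Damage reduces health, then triggers pelvis-down physics with a hit impulse.
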(event Custom|ChasePlayerEvent
  (bind _returnvalue (Transformation|GetActorLocation))
  (bind _returnvalue_2 (Game|GetPlayerCharacter 0))
  (bind _returnvalue_3 (Transformation|GetActorLocation _returnvalue_2))
  ;[1 1 1] Chase Player
  (if (not (Variables|Default|GetJumping))
    (if (Variables|Default|GetCanMove)
      (Pawn|Input|AddMovementInput (Math|Vector|GetUnitDirection(Vector) _returnvalue _returnvalue_3) 1.0 false)
      (Transformation|SetActorRotation (Math|Rotator|MakeRotator 0.0 0.0 (.yaw (Math|Rotator|FindLookatRotation _returnvalue _returnvalue_3)))))))

(event Custom|Attack%20Player
  ;[1 1 1] Attack Player
  (if (not (Variables|Default|GetAttacking))
    (Variables|Default|SetAttacking true)
    (Animation|Montage|PlayMontage (Variables|Character|GetMesh) (.OutItem (Utilities|Array|Random (Variables|Default|GetAttackMontage)))
      (:OnCompleted
        (if (Variables|Default|GetNearPlayer)
          _
          (else
            (Utilities|FlowControl|Delay 1.0)))
        (Variables|Default|SetAttacking false)))))

(event EventTick
  (params (DeltaSeconds :type Float%20%28single-precision%29))
  ;[1 1 1] Event Tick
  (CallFunction|UpdateCharacterSpeed)
  (CallFunction|Tracers)
  (switch Utilities|FlowControl|Switch|SwitchonZombieState (Variables|Default|GetZombieState)
    (:NewEnumerator0
      (CallFunction|ZombieIdle))
    (:NewEnumerator1
      (CallFunction|ChasePlayerEvent)
      (if (Variables|Default|GetNearPlayer)
        (CallFunction|AttackPlayer)))
    (:NewEnumerator3
      (if (not (Class|Actor|WasRecentlyRendered 22.0))
        (Actor|DestroyActor)))))

(event Custom|Tracers
  (bind _returnvalue (Transformation|GetActorLocation))
  (bind _returnvalue_2 (Transformation|GetActorLocation))
  (bind _returnvalue_3 (Game|GetPlayerCharacter 0))
  (bind _capsulecomponent (Variables|Collision|GetCapsuleComponent))
  (bind _returnvalue_4 (- (.z _returnvalue) 5e+01))
  (bind _returnvalue_5 (- (.z _returnvalue_2) 5e+01))
  (bind _returnvalue_6 (Math|Vector|MakeVector (.x _returnvalue) (.y _returnvalue) _returnvalue_4))
  (bind _returnvalue_7 (Math|Vector|MakeVector (.x _returnvalue_2) (.y _returnvalue_2) _returnvalue_5))
  (if (Utilities|Enum|NotEqual(Enum) (Variables|Default|GetZombieState) "NewEnumerator3")
    (Utilities|FlowControl|Sequence
      (:then_0
        (if (Variables|Default|GetJumping)
          (Transformation|SetWorldRotation (Variables|Collision|GetCapsuleComponent) (Math|Rotator|MakeRotator 0.0 0.0 (.yaw (Transformation|GetWorldRotation (Variables|Collision|GetCapsuleComponent)))) false false)
          (else
            (bind (_outhit _returnvalue_8) (Collision|SphereTraceByChannel _returnvalue_7 (+ _returnvalue_7 (* (Math|Vector|GetForwardVector (Transformation|GetActorRotation)) 6e+01)) 1e+01 "TraceTypeQuery4" false (Utilities|Array|MakeArray self) "None"))
            (if _returnvalue_8
              (Variables|Default|SetMantleWallLocation (.Location (Collision|BreakHitResult _outhit)))
              (Variables|Default|SetMantleWallNormal (.ImpactNormal (Collision|BreakHitResult _outhit)))
              (bind (_outhit_2 _returnvalue_9) (Collision|SphereTraceByChannel (Math|Vector|MakeVector (.X (Math|Vector|BreakVector (+ (* (Variables|Default|GetMantleWallNormal) -3e+01) (Variables|Default|GetMantleWallLocation)))) (.Y (Math|Vector|BreakVector (+ (* (Variables|Default|GetMantleWallNormal) -3e+01) (Variables|Default|GetMantleWallLocation)))) (+ (.Z (Math|Vector|BreakVector (+ (* (Variables|Default|GetMantleWallNormal) -3e+01) (Variables|Default|GetMantleWallLocation)))) 2e+02)) (Math|Vector|MakeVector (.X (Math|Vector|BreakVector (+ (* (Variables|Default|GetMantleWallNormal) -3e+01) (Variables|Default|GetMantleWallLocation)))) (.Y (Math|Vector|BreakVector (+ (* (Variables|Default|GetMantleWallNormal) -3e+01) (Variables|Default|GetMantleWallLocation)))) (+ (.Z (Math|Vector|BreakVector (+ (* (Variables|Default|GetMantleWallNormal) -3e+01) (Variables|Default|GetMantleWallLocation)))) -2e+01)) 1e+01 "TraceTypeQuery4" false (Utilities|Array|MakeArray self) "None"))
              (if _returnvalue_9
                (Variables|Default|SetMantleWallHeight (.Location (Collision|BreakHitResult _outhit_2)))
                (if (< (Math|Float|Absolute(Float) (- (Math|Float|Absolute(Float) (.z (Transformation|GetSocketLocation (Variables|Character|GetMesh) "root"))) (Math|Float|Absolute(Float) (.Z (Math|Vector|BreakVector (.Location (Collision|BreakHitResult _outhit_2))))))) 1.5e+02)
                  (Variables|Default|SetMantleMontage "/Game/GameFiles/Zombies/Animations/Mantle_1m_LH_Montage.Mantle_1m_LH_Montage")
                  (Variables|Default|SetPositionOffset -2e+01)
                  (Variables|Default|SetJumping true :!label _label)
                  (Utilities|FlowControl|Delay (Math|Random|RandomFloatinRange 0.0 2.0))
                  (Collision|SetCollisionEnabled (Variables|Collision|GetCapsuleComponent) "NoCollision")
                  (Transformation|SetWorldLocation _capsulecomponent (Math|Vector|MakeVector (.x (+ (* (Variables|Default|GetMantleWallNormal) 45.0) (Variables|Default|GetMantleWallLocation))) (.y (+ (* (Variables|Default|GetMantleWallNormal) 45.0) (Variables|Default|GetMantleWallLocation))) (.z (Transformation|GetWorldLocation (Variables|Collision|GetCapsuleComponent)))) false false)
                  (Transformation|SetWorldRotation _capsulecomponent (Math|Rotator|MakeRotator 0.0 0.0 (.yaw (Math|Rotator|FindLookatRotation (Transformation|GetActorLocation) (Variables|Default|GetMantleWallLocation)))) false false)
                  (Animation|Montage|PlayMontage (Variables|Character|GetMesh) (Variables|Default|GetMantleMontage)
                    (:then
                      (Pawn|Components|CharacterMovement|SetMovementMode (Variables|Character|GetCharacterMovement) "MOVE_Flying" 0))
                    (:OnCompleted
                      (Pawn|Components|CharacterMovement|SetMovementMode (Variables|Character|GetCharacterMovement) "MOVE_Walking" 0)
                      (Collision|SetCollisionEnabled (Variables|Collision|GetCapsuleComponent) "QueryAndPhysics")
                      (Utilities|FlowControl|Delay 0.2)
                      (Variables|Default|SetJumping false)))
                  (elif (not (> (Math|Float|Absolute(Float) (- (Math|Float|Absolute(Float) (.z (Transformation|GetSocketLocation (Variables|Character|GetMesh) "root"))) (Math|Float|Absolute(Float) (.Z (Math|Vector|BreakVector (.Location (Collision|BreakHitResult _outhit_2))))))) 2.2e+02))
                    (Variables|Default|SetMantleMontage "/Game/GameFiles/Zombies/Animations/Mantle2M_Montage.Mantle2M_Montage")
                    (Variables|Default|SetPositionOffset -1e+02)
                    (goto _label))))))))
      (:then_1
        (bind (_outhit_3 _returnvalue_10) (Collision|SphereTraceByChannel _returnvalue_6 (+ _returnvalue_6 (* (Math|Vector|GetForwardVector (Transformation|GetActorRotation)) 8e+01)) 2e+01 "TraceTypeQuery1" false 0 "None"))
        (if _returnvalue_10
          (if (== (.HitActor (Collision|BreakHitResult _outhit_3)) _returnvalue_3)
            (if (< (Math|Vector|VectorLength (- (Transformation|GetActorLocation) (Transformation|GetActorLocation _returnvalue_3))) 8e+01)
              (Variables|Default|SetNearPlayer true))
            (else
              (Variables|Default|SetNearPlayer false :!label _label_2)))
          (else
            (goto _label_2)))))))

(event Custom|ZombieIdle
  (bind _returnvalue (Transformation|GetActorLocation))
  (bind _returnvalue_2 (Transformation|GetActorLocation))
  (if (Variables|Default|GetCanRoam)
    (if (Variables|Default|GetCanMove)
      (if (Variables|Default|GetIsRoaming)
        (Pawn|Input|AddMovementInput (Math|Vector|GetUnitDirection(Vector) _returnvalue_2 (stale _output_get)) 1.0 true)
        (if (Math|Vector|Equal(Vector) (Transformation|GetActorLocation) (Variables|Default|GetRoamLocation) 5e+01)
          (Variables|Default|SetIsRoaming false))
        (else
          (Utilities|FlowControl|Delay (Math|Random|RandomFloatinRange 2.0 6.0))
          (if (Utilities|Enum|Equal(Enum) (Variables|Default|GetZombieState) "NewEnumerator0")
            (Variables|Default|SetIsRoaming true)
            (bind _output_get (Variables|Default|SetRoamLocation (Math|Vector|MakeVector (+ (.x _returnvalue) (Math|Random|RandomFloatinRange -3e+02 3e+02)) (+ (.y _returnvalue) (Math|Random|RandomFloatinRange -3e+02 3e+02)) (.z _returnvalue))))
            (bind _alpha (Timeline|RotateTimeline PlayFromStart)
              (:Update
                (Transformation|SetActorRotation (Math|Rotator|Lerp(Rotator) (Transformation|GetActorRotation) (Math|Rotator|FindLookatRotation _returnvalue_2 _output_get) _alpha true))))))))))

(event EventDamage
  (params (Damage :type Float%20%28double-precision%29) (DamageType :type DamageTyoe%20Enum :default "NewEnumerator0") (BoneName :type Name :default "None") (ImpulseValue :type Vector :default "0, 0, 0") (HitLocation :type Vector :default "0, 0, 0"))
  (Variables|Default|SetLocalDamage Damage)
  (if (not (Utilities|Enum|Equal(Enum) (Variables|Default|GetZombieState) "NewEnumerator3"))
    (bind _output_get (Variables|Default|SetHealth (- (Variables|Default|GetHealth) (Variables|Default|GetLocalDamage))))
    (if (<= _output_get 0.0)
      (Variables|Default|SetZombieState "NewEnumerator3")
      (CallFunction|RagdollStart)
      (Physics|AddImpulseatLocation (Variables|Character|GetMesh) ImpulseValue HitLocation BoneName))))

(fn ConstructionScript
  (Components|SkinnedMesh|SetSkinnedAssetandUpdate (Variables|Character|GetMesh) (.OutItem (Utilities|Array|Random (Variables|Default|GetNew%20Mesh))) true))

(fn UpdateCharacterSpeed
  (switch Utilities|FlowControl|Switch|SwitchonZombieState (Variables|Default|GetZombieState)
    (:NewEnumerator0
      (if (Variables|Default|GetCanRoam)
        (Variables|/Script/Engine.CharacterMovementComponent|SetMaxWalkSpeed (Variables|Character|GetCharacterMovement) 45.0 :!label _label)
        (else
          (Variables|/Script/Engine.CharacterMovementComponent|SetMaxWalkSpeed (Variables|Character|GetCharacterMovement) 0.0))))
    (:NewEnumerator1
      (if (Variables|Default|GetNearPlayer)
        (goto _label)
        (else
          (Variables|/Script/Engine.CharacterMovementComponent|SetMaxWalkSpeed (Variables|Character|GetCharacterMovement) 4e+02))))))

(fn RagdollStart
  (bind _mesh (Variables|Character|GetMesh))
  (Utilities|FlowControl|Sequence
    (:then_0
      ;[1 1 1] Step 1: Clear the Character Movement Mode and set teh Movement State to Ragdoll
      (Pawn|Components|CharacterMovement|SetMovementMode (Variables|Character|GetCharacterMovement) "MOVE_None" 0))
    (:then_1
      ;[1 1 1] Step 2: Disable capsule collision and enable mesh physics simulation starting from the pelvis.
      (Collision|SetCollisionEnabled (Variables|Collision|GetCapsuleComponent) "NoCollision")
      (Collision|SetCollisionObjectType _mesh "ECC_PhysicsBody")
      (Collision|SetCollisionEnabled _mesh "QueryAndPhysics")
      (Class|SkeletalMeshComponent|SetAllBodiesBelowSimulatePhysics _mesh (Utilities|Name|MakeLiteralName "pelvis") true true))))

(fn Properties
  (return (Variables|Default|GetIsDead) (Variables|Default|GetHealth) (Variables|Default|GetZombieState) (Variables|Default|GetCanRoam)))