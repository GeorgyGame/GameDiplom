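; BP_GrappleLine is a grapple line actor that hands off to the player's hook cable when the line is retracted.
; It caches the player character on BeginPlay.
; RetractCable hides its own cable, attaches the start of the player's HookCable and drives that cable's length with a timeline.
; When the timeline finishes, it attaches the cable end to the player's hip rope socket and destroys itself.
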(event Custom|RetractCable
  (bind _playerref (Variables|Default|GetPlayerRef))
  (bind _hookcable (Variables|/Game/AdvancedLocomotionV4/Blueprints/CharacterLogic/PlayerCharacter.PlayerCharacter_C|GetHookCable _playerref))
  (Rendering|SetVisibility (Variables|Default|GetCableComponent) false false)
  (Variables|/Script/CableComponent.CableComponent|SetbAttachStart (Variables|/Game/AdvancedLocomotionV4/Blueprints/CharacterLogic/PlayerCharacter.PlayerCharacter_C|GetHookCable (Variables|Default|GetPlayerRef)) true)
  (bind _cablelength (Timeline|Retract PlayFromStart)
    (:Update
      (Variables|/Script/CableComponent.CableComponent|SetCableLength (Variables|/Game/AdvancedLocomotionV4/Blueprints/CharacterLogic/PlayerCharacter.PlayerCharacter_C|GetHookCable (Variables|Default|GetPlayerRef)) _cablelength))
    (:Finished
      (Variables|/Script/CableComponent.CableComponent|SetbAttachEnd _hookcable true)
      (Class|CableComponent|SetAttachEndto _hookcable _playerref "Mesh" "RopeHipSocket")
      (Actor|DestroyActor))))

(event EventBeginPlay
  (bind _asplayer_character (Utilities|Casting|CastToPlayerCharacter (Game|GetPlayerCharacter 0)))
  (Variables|Default|SetPlayerRef _asplayer_character))

(fn ConstructionScript)