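; Base ammo pickup actor that gives the player ammo for a specific weapon through an interact prompt.
; Pickup binds AmmoPickup to the player's interact dispatcher and, if the interact HUD is hidden, shows the weapon-type prompt for two seconds before clearing all interact bindings.
; On interact, AmmoPickup passes the weapon and count to the player, destroying the actor and removing the prompt only on success.
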(event Custom|AmmoPickup
  (bind _successful (Default|AmmoPickup (Variables|Default|GetPlayerRef) (Variables|Default|GetWeapon) (Variables|Default|GetAmmoCount)))
  (if _successful
    (Actor|DestroyActor)
    (Widget|RemovefromParent (Variables|/Game/AdvancedLocomotionV4/Blueprints/CharacterLogic/PlayerCharacter.PlayerCharacter_C|GetInteractHUD_Ref (Variables|Default|GetPlayerRef)))))

(event EventBeginPlay
  ;[1 1 1] Player Ref
  (bind _asplayer_character (Utilities|Casting|CastToPlayerCharacter (Game|Player|GetPlayerPawn 0)))
  (Variables|Default|SetPlayerRef _asplayer_character))

(event EventPickup
  (bind _playerref (Variables|Default|GetPlayerRef))
  (bind _playerref_2 (Variables|Default|GetPlayerRef))
  (bind _interacthud_ref (Variables|/Game/AdvancedLocomotionV4/Blueprints/CharacterLogic/PlayerCharacter.PlayerCharacter_C|GetInteractHUD_Ref _playerref))
  (EventDispatchers|BindEventtoInteract _playerref (delegate Custom|AmmoPickup))
  (if (not (UserInterface|Viewport|IsinViewport _interacthud_ref))
    (Default|UpdateInteractText _interacthud_ref (Utilities|String|Append "Pick " (Utilities|String|EnumtoString (Variables|Default|GetWeaponType)) " Ammo"))
    (UserInterface|Viewport|AddtoViewport _interacthud_ref 0)
    (Utilities|FlowControl|Delay 2.0)
    (EventDispatchers|UnbindallEventsfromInteract _playerref_2)
    (Widget|RemovefromParent (Variables|/Game/AdvancedLocomotionV4/Blueprints/CharacterLogic/PlayerCharacter.PlayerCharacter_C|GetInteractHUD_Ref _playerref_2))))

(fn ConstructionScript)