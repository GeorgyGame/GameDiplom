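; MedKit pickup actor that adds a medkit to the player's inventory, up to the player's maximum.
; Pickup binds to the player's Interact dispatcher and shows a prompt, then after a two-second delay unbinds all Interact listeners and hides it.
; Interacting increments the count, updates the health HUD and weapon menu, enables the menu's top-left button, destroys the actor and removes the prompt.
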(event Custom|Pickup_Event
  (bind _playerref (Variables|Default|GetPlayerRef))
  (bind _playerref_2 (Variables|Default|GetPlayerRef))
  (bind _playerref_3 (Variables|Default|GetPlayerRef))
  (bind _playercontroller_ref (Variables|/Game/AdvancedLocomotionV4/Blueprints/CharacterLogic/PlayerCharacter.PlayerCharacter_C|GetPlayerController_Ref _playerref_3))
  (bind _weaponmenuhref (Variables|/Game/AdvancedLocomotionV4/Blueprints/CharacterLogic/ALS_Player_Controller.ALS_Player_Controller_C|GetWeaponMenuHRef _playercontroller_ref))
  (if (< (Variables|/Game/AdvancedLocomotionV4/Blueprints/CharacterLogic/PlayerCharacter.PlayerCharacter_C|GetMedKit _playerref) (Variables|/Game/AdvancedLocomotionV4/Blueprints/CharacterLogic/PlayerCharacter.PlayerCharacter_C|GetMaxMedKit _playerref))
    (bind _output_get (Variables|/Game/AdvancedLocomotionV4/Blueprints/CharacterLogic/PlayerCharacter.PlayerCharacter_C|SetMedKit _playerref_2 (+ (Variables|/Game/AdvancedLocomotionV4/Blueprints/CharacterLogic/PlayerCharacter.PlayerCharacter_C|GetMedKit _playerref_2) 1)))
    (Default|UpdateHealthHud (Variables|/Game/GameFiles/Blueprint/UI/MainHud.MainHud_C|GetHealthHUD (Variables|/Game/AdvancedLocomotionV4/Blueprints/CharacterLogic/PlayerCharacter.PlayerCharacter_C|GetMainHudRef _playerref_3)) 0.0 0.0 0.0 "NewEnumerator2" _output_get 0 0.0)
    (Rendering|Components|TextRender|SetText (Variables|/Game/GameFiles/Blueprint/UI/WeaponMenu/WeaponMenu.WeaponMenu_C|GetMedKit _weaponmenuhref) (Utilities|Text|ToText(Integer) _output_get))
    (Widget|SetIsEnabled (Variables|/Game/GameFiles/Blueprint/UI/WeaponMenu/WeaponMenu.WeaponMenu_C|GetTopLeftBtn _weaponmenuhref) true)
    (Actor|DestroyActor)
    (Widget|RemovefromParent (Variables|/Game/AdvancedLocomotionV4/Blueprints/CharacterLogic/PlayerCharacter.PlayerCharacter_C|GetInteractHUD_Ref (Variables|Default|GetPlayerRef)))))

(event EventBeginPlay
  ;[1 1 1] Player Ref
  (bind _asplayer_character (Utilities|Casting|CastToPlayerCharacter (Game|Player|GetPlayerPawn 0)))
  (Variables|Default|SetPlayerRef _asplayer_character))

(event EventPickup
  (bind _playerref (Variables|Default|GetPlayerRef))
  (bind _playerref_2 (Variables|Default|GetPlayerRef))
  (bind _interacthud_ref (Variables|/Game/AdvancedLocomotionV4/Blueprints/CharacterLogic/PlayerCharacter.PlayerCharacter_C|GetInteractHUD_Ref _playerref))
  (EventDispatchers|BindEventtoInteract _playerref (delegate Custom|Pickup_Event))
  (if (not (UserInterface|Viewport|IsinViewport _interacthud_ref))
    (Default|UpdateInteractText _interacthud_ref (Utilities|String|Append "Pick " "Medkits"))
    (UserInterface|Viewport|AddtoViewport _interacthud_ref 0)
    (Utilities|FlowControl|Delay 2.0)
    (EventDispatchers|UnbindallEventsfromInteract _playerref_2)
    (Widget|RemovefromParent (Variables|/Game/AdvancedLocomotionV4/Blueprints/CharacterLogic/PlayerCharacter.PlayerCharacter_C|GetInteractHUD_Ref _playerref_2))))

(fn ConstructionScript)