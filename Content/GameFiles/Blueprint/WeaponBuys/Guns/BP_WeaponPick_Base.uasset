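; Base weapon pickup actor that gives the player a weapon with its magazine and bag ammo when they interact.
; Pickup shows the weapon type on the player's interact HUD and binds PickUpEvent to the Interact dispatcher, clearing all of that dispatcher's bindings after a short delay.
; PickUpEvent asks the player to spawn the weapon at its socket, then destroys the pickup and removes the prompt on success.
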(event Custom|PickUpEvent
  (bind _successful (Default|SpawnWeapon (Variables|Reference|GetPlayerRef) (Variables|Default|GetWeapon) (Variables|Default|GetWeaponSocket) (Variables|Default|GetMagAmmo) (Variables|Default|GetBagAmmo)))
  (if _successful
    (Actor|DestroyActor)
    (Widget|RemovefromParent (Variables|/Game/AdvancedLocomotionV4/Blueprints/CharacterLogic/PlayerCharacter.PlayerCharacter_C|GetInteractHUD_Ref (Variables|Reference|GetPlayerRef)))))

(event EventBeginPlay
  ;[1 1 1] Begin Play
  (bind _asplayer_character (Utilities|Casting|CastToPlayerCharacter (Game|Player|GetPlayerPawn 0)))
  (Variables|Reference|SetPlayerRef _asplayer_character))

(event EventPickup
  (bind _playerref (Variables|Reference|GetPlayerRef))
  (bind _interacthud_ref (Variables|/Game/AdvancedLocomotionV4/Blueprints/CharacterLogic/PlayerCharacter.PlayerCharacter_C|GetInteractHUD_Ref _playerref))
  (EventDispatchers|BindEventtoInteract _playerref (delegate Custom|PickUpEvent))
  (if (UserInterface|Viewport|IsinViewport _interacthud_ref)
    _
    (else
      (UserInterface|Viewport|AddtoViewport _interacthud_ref 0)))
  (Default|UpdateInteractText _interacthud_ref (Utilities|String|Append "Pick " (Utilities|String|EnumtoString (Variables|Default|GetWeaponType))))
  (Utilities|FlowControl|Delay 0.2)
  (EventDispatchers|UnbindallEventsfromInteract (Variables|Reference|GetPlayerRef)))

(fn ConstructionScript)