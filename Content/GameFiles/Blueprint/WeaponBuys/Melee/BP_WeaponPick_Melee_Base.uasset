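; Base Blueprint for melee weapon pickups that give the player a weapon on interact.
; BeginPlay caches the player character, and Pickup binds its interact event to PickUp_Event.
; If the interact HUD is not already showing, it displays a weapon-type prompt, then after a short delay clears all interact bindings and hides it.
; PickUp_Event has the player spawn the weapon and, on success, destroys the pickup and removes the prompt.
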(event Custom|PickUp_Event
  (bind _successfull (Default|SpawnMeleeWeapon (Variables|Reference|GetPlayerRef) (Variables|Default|GetWeapon)))
  (if _successfull
    (Actor|DestroyActor)
    (Widget|RemovefromParent (Variables|/Game/AdvancedLocomotionV4/Blueprints/CharacterLogic/PlayerCharacter.PlayerCharacter_C|GetInteractHUD_Ref (Variables|Reference|GetPlayerRef)))))

(event EventBeginPlay
  ;[1 1 1] Begin Play
  (bind _asplayer_character (Utilities|Casting|CastToPlayerCharacter (Game|Player|GetPlayerPawn 0)))
  (Variables|Reference|SetPlayerRef _asplayer_character))

(event EventPickup
  (bind _playerref (Variables|Reference|GetPlayerRef))
  (bind _playerref_2 (Variables|Reference|GetPlayerRef))
  (bind _interacthud_ref (Variables|/Game/AdvancedLocomotionV4/Blueprints/CharacterLogic/PlayerCharacter.PlayerCharacter_C|GetInteractHUD_Ref _playerref_2))
  (EventDispatchers|BindEventtoInteract _playerref_2 (delegate Custom|PickUp_Event))
  (if (not (UserInterface|Viewport|IsinViewport _interacthud_ref))
    (Default|UpdateInteractText _interacthud_ref (Utilities|String|Append "Pick " (Utilities|String|EnumtoString (Variables|Default|GetWeaponType))))
    (UserInterface|Viewport|AddtoViewport _interacthud_ref 0)
    (Utilities|FlowControl|Delay 2.0)
    (EventDispatchers|UnbindallEventsfromInteract _playerref)
    (Widget|RemovefromParent (Variables|/Game/AdvancedLocomotionV4/Blueprints/CharacterLogic/PlayerCharacter.PlayerCharacter_C|GetInteractHUD_Ref _playerref))))

(fn ConstructionScript)