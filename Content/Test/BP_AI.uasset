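; BP_AI is a test AI enemy character that detects the player and performs melee attacks.
; Pawn sensing sets a "seen player" Blackboard flag on its AI controller when it spots a PlayerCharacter; the flag is never cleared here.
; An AttackPlayer event sphere-traces forward with debug drawing and, on hitting the player, plays a random half-speed montage and immediately sends damage through a DamageMessage call.
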(event OnSeePawn(PawnSensing)
  (params (Pawn :type Pawn%20Object%20Reference))
  (Utilities|Casting|CastToPlayerCharacter Pawn)
  (AI|Components|Blackboard|SetValueasBool (AI|GetBlackboard (AI|GetAIController self)) (Utilities|Name|MakeLiteralName "hasSeenPlayer?") true))

(event Custom|AttackPlayer
  (bind _returnvalue (Transformation|GetActorLocation))
  (bind (_outhit _returnvalue_2) (Collision|SphereTraceForObjects _returnvalue (+ _returnvalue (* (Math|Vector|GetForwardVector (Transformation|GetActorRotation)) 2.5e+02)) 1e+02 (Utilities|Array|MakeArray "ObjectTypeQuery3") false 0 "ForDuration"))
  (if _returnvalue_2
    (Utilities|Casting|CastToPlayerCharacter (.HitActor (Collision|BreakHitResult _outhit)))
    (Animation|PlayAnimMontage (.OutItem (Utilities|Array|Random (Variables|Default|GetAnim%20Montage))) 0.5 "None")
    (Class|DamageInterface|Damage(Message) (.HitActor (Collision|BreakHitResult _outhit)) 2e+01 "NewEnumerator3" "None" "0, 0, 0" "0, 0, 0")))

(event EventBeginPlay)

(event Collision|EventActorBeginOverlap
  (params (OtherActor :type Actor%20Object%20Reference)))

(event EventTick
  (params (DeltaSeconds :type Float%20%28single-precision%29)))

(fn ConstructionScript)